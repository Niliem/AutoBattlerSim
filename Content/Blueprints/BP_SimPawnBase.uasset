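; BP_SimPawnBase is a base pawn that visualizes simulation events: health changes, attacks, movement and death.
; Health updates set the text percentage and the sphere's dynamic material emissive, then play a scale-pulse timeline.
; Attacks aim and animate the arrow, FinishMovement quickly lerps the actor to its target, and death hides it.
; StartMovement, marked TODO, only sets rotation and timeline play rate, as its position lerp is never triggered.
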(event `self.ReceiveBeginPlay`
  (bind _returnvalue (`PrimitiveComponent.CreateDynamicMaterialInstance` (`self.Sphere`) 0 (`PrimitiveComponent.GetMaterial` (`self.Sphere`) 0) "None"))
  (set `self.MaterialInstance` _returnvalue))

(event `CombatSimInterface.UpdateHealth`
  (params (HealthPercent :type "Float (single-precision)"))
  (`TextRenderComponent.K2_SetText` (`self.TextRender`) (`KismetTextLibrary.Conv_DoubleToText` (* HealthPercent 100.0) "HalfToEven"))
  (bind _materialinstance (`self.MaterialInstance`)
    (:`then`
      (`MaterialInstanceDynamic.SetScalarParameterValue` _materialinstance "EmissiveAlpha" HealthPercent)
      (bind (_direction _alpha) (`Timeline|HitAnmim` :!via `PlayFromStart`)
        (:`Update`
          (`SceneComponent.SetRelativeScale3D` (`self.Sphere`) (`KismetMathLibrary.VLerp` (1.0 1.0 1.0) (1.0 1.1 1.0) _alpha)))))
    (:`else`)))

(event `CombatSimInterface.Dead`
  (`self.SetActorHiddenInGame` true))

(event `CombatSimInterface.Attack`
  (params (TargetPosition :type "Vector Structure"))
  (bind _arrow (`self.Arrow`))
  (`SceneComponent.K2_SetWorldRotation` (`self.Arrow`) (`KismetMathLibrary.FindLookAtRotation` (`SceneComponent.K2_GetComponentLocation` (`self.Arrow`)) TargetPosition) false false)
  (bind (_direction _alpha) (`Timeline|AttackAnimation` :!via `PlayFromStart`)
    (:`Update`
      (`SceneComponent.K2_SetRelativeLocation` _arrow (`KismetMathLibrary.VLerp` (0.0 -20.0 49.0) (* (`SceneComponent.GetForwardVector` _arrow) (50.0 -20.0 40.0)) _alpha) false false))))

(event `CombatSimInterface.FinishMovement`
  (params (TargetPosition :type "Vector Structure"))
  (set `self.OriginalLocation` (`self.K2_GetActorLocation`))
  (`TimelineComponent.SetPlayRate` (`self.CustomMovement`) 3.0)
  (bind (_direction _alpha) (`Timeline|CustomMovement` :!via `PlayFromStart`)
    (:`Update`
      (`self.K2_SetActorLocation` (`KismetMathLibrary.VLerp` (`self.OriginalLocation`) TargetPosition _alpha) false true))))

(event `CombatSimInterface.StartMovement`
  (params (StartPosition :type "Vector Structure") (TargetPosition :type "Vector Structure") (Duration :type "Float (single-precision)"))
  ;[1 1 1] TODO: Fix)
  (`self.K2_SetActorRotation` (`KismetMathLibrary.FindLookAtRotation` StartPosition TargetPosition))
  (`TimelineComponent.SetPlayRate` (`self.MovementAnimation`) (`KismetMathLibrary.SafeDivide` 1.0 Duration)))

(fn `UserConstructionScript`)